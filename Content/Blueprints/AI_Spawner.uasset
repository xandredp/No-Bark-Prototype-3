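; AI spawner actor that releases escalating waves of AI_Character enemies at a fixed point in the level.
; BeginPlay sets the starting wave size and starts a looping timer that calls SpawnWave by name, so the first wave follows a delay.
; SpawnWave spawns the batch at the Arrow component's location, adjusting for collisions but always spawning, then raises the next wave's size by a fixed step with no upper limit.
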(event EventBeginPlay
  (Variables|Default|SetMaxSpawnNumber 5)
  (Utilities|Time|SetTimerbyFunctionName 0 "SpawnWave" 2e+01 true))

(event Collision|EventActorBeginOverlap
  (params (OtherActor :type Actor%20Object%20Reference)))

(event EventTick
  (params (DeltaSeconds :type Float%20%28single-precision%29)))

(fn ConstructionScript)

(fn SpawnWave
  (for _index (range 0 (Variables|Default|GetMaxSpawnNumber))
    (Game|SpawnActorfromClass "/Game/AI/AI_Character.AI_Character_C" (Math|Conversions|ToTransform(Vector) (Transformation|GetWorldLocation (Variables|Default|GetArrow))) "AdjustIfPossibleButAlwaysSpawn" 0 0))
  (Variables|Default|SetMaxSpawnNumber (+ (Variables|Default|GetMaxSpawnNumber) 5)))